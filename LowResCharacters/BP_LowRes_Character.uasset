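; BP_LowRes_Character is a low-resolution character that gets a randomized look, with no gameplay logic in its event graph.
; Its construction script calls SetSKM, which picks a random index into the SKM mesh array and applies that skeletal mesh along with the Anim Blueprint at the same index in the parallel ABP array.
; The pick is unseeded, so it can change whenever the construction script reruns.
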(event EventBeginPlay)

(event Collision|EventActorBeginOverlap
  (params (OtherActor :type Actor%20Object%20Reference)))

(event EventTick
  (params (DeltaSeconds :type Float%20%28single-precision%29)))

(fn ConstructionScript
  (CallFunction|SetSKM))

(fn SetSKM
  (bind _mesh (Variables|Character|GetMesh))
  (LocalVariables|SetRandIdx (Math|Random|RandomInteger (Utilities|Array|Length (Variables|Default|GetSKM))))
  (Class|SkeletalMeshComponent|SetAnimClass _mesh (Utilities|Array|Get(acopy) (Variables|Default|GetABP) (LocalVariables|GetRandIdx)))
  (Components|SkinnedMesh|SetSkinnedAssetandUpdate _mesh (Utilities|Array|Get(acopy) (Variables|Default|GetSKM) (LocalVariables|GetRandIdx)) true))